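; Player camera manager that drives a lagged follow camera for characters implementing CameraSetup_BPI, falling back to parent camera logic otherwise.
; Each update reads socket, FOV and offset targets from that interface, then interpolates them and the control rotation.
; The socket lags independently per yaw-relative axis, with velocity-scaled softer vertical lag while falling.
; A sphere trace against WorldStatic pulls the offset camera in front of obstructions.
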(event EventBeginPlay
  (CallFunction|UpdateActorInfo)
  (Utilities|UpdateCameraRotation
    (:Valid
      (Variables|Socket|SetTargetSocket (Variables|Socket|GetTargetSocket_Target)))))

(fn ConstructionScript)

(fn BlueprintUpdateCamera
  (params (CameraTarget :type Actor%20Object%20Reference))
  (Utilities|UpdateCameraRotation
    (:Valid
      (return (Variables|Camera|GetCameraLocation) (Variables|Camera|GetCameraRotation) (Variables|Default|GetFOV) true))
    (:Invalid
      (bind (_newcameralocation _newcamerarotation _newcamerafov _returnvalue) (|CallParentFunction CameraTarget))
      (return _newcameralocation _newcamerarotation _newcamerafov _returnvalue))))

(fn CalculateAxisIndependentLag
  (params (CurrentLocation :type Vector) (TargetLocation :type Vector) (CameraRotation :type Rotator) (LagSpeeds :type Vector) (DeltaTime :type Float%20%28double-precision%29))
  (bind _returnvalue (Math|Rotator|MakeRotator 0.0 0.0 (.yaw CameraRotation)))
  (bind _returnvalue_2 (Math|Vector|UnrotateVector TargetLocation _returnvalue))
  (bind _returnvalue_3 (Math|Vector|UnrotateVector CurrentLocation _returnvalue))
  (return (Math|Vector|RotateVector (Math|Vector|MakeVector (Math|Interpolation|FInterpTo (.x _returnvalue_3) (.x _returnvalue_2) DeltaTime (.x LagSpeeds)) (Math|Interpolation|FInterpTo (.y _returnvalue_3) (.y _returnvalue_2) DeltaTime (.y LagSpeeds)) (Math|Interpolation|FInterpTo (.z _returnvalue_3) (.z _returnvalue_2) DeltaTime (.z LagSpeeds))) _returnvalue)))

(fn UpdateActorInfo
  (bind _ascharacter (Utilities|Casting|CastToCharacter (Pawn|GetControlledPawn (Game|Player|GetOwningPlayerController)))
    (:then
      (bind _output_get (Variables|Default|SetCharacter _ascharacter))
      (Variables|Default|SetCharacterMovement (Variables|/Script/Engine.Character|GetCharacterMovement _output_get))
      (Utilities|IsValid _output_get
        (:Is%20Valid
          (if (Utilities|DoesObjectImplementInterface _output_get "/Game/Blueprints/Camera/CameraSetup_BPI.CameraSetup_BPI_C")
            (bind _ascamera_setup_bpi (Utilities|Casting|CastToCameraSetup_BPI (Variables|Default|GetCharacter))
              (:then
                (Variables|Default|SetCameraSetup _ascamera_setup_bpi)
                (Variables|Default|SetIsValid true))
              (:CastFailed
                (Variables|Default|SetIsValid false :!label _label)))
            (else
              (goto _label))))
        (:Is%20Not%20Valid
          (goto _label))))
    (:CastFailed
      (goto _label))))

(fn UpdateParameters
  (bind _socket (Default|GetViewSocket (Variables|Default|GetCameraSetup)))
  (Variables|Socket|SetTargetSocket_Target _socket)
  (bind (_fov _offset) (Default|GetCameraParameters (Variables|Default|GetCameraSetup)))
  (Variables|Default|SetFOV_Target _fov)
  (Variables|Camera|SetCameraOffset_Target _offset))

(fn InterpolateFOV
  (Variables|Default|SetFOV (Math|Interpolation|FInterpTo (Variables|Default|GetFOV) (Variables|Default|GetFOV_Target) (Utilities|Time|GetWorldDeltaSeconds) (Variables|Default|GetFOV_LagSpeed))))

(fn InterpolateCameraRotation
  (Variables|Camera|SetCameraRotation (Math|Interpolation|RInterpTo (Camera|GetCameraRotation) (Pawn|GetControlRotation (Game|Player|GetOwningPlayerController) :!class /Script/Engine.Controller) (Utilities|Time|GetWorldDeltaSeconds) (Variables|Camera|GetCameraRotation_LagSpeed))))

(fn CalculateSocketTransform
  (bind _targetsocket_lagspeed (Variables|Socket|GetTargetSocket_LagSpeed))
  (Variables|Socket|SetTargetSocket (Math|Transform|MakeTransform (CallFunction|CalculateAxisIndependentLag (.location (Variables|Socket|GetTargetSocket)) (.location (Variables|Socket|GetTargetSocket_Target)) (Variables|Camera|GetCameraRotation) (Math|Vector|MakeVector (.x _targetsocket_lagspeed) (.y _targetsocket_lagspeed) (* (.z _targetsocket_lagspeed) (Math|Float|SelectFloat (Math|Float|Clamp(Float) (- (/ (Math|Float|Absolute(Float) (.z (Variables|/Script/Engine.MovementComponent|GetVelocity (Variables|Default|GetCharacterMovement)))) 1e+03) 0.3) 0.01 0.3) 1.0 (AI|Components|NavMovement|IsFalling (Variables|Default|GetCharacterMovement))))) (Utilities|Time|GetWorldDeltaSeconds)) (.rotation (Variables|Socket|GetTargetSocket)))))

(fn CalculateCameraLocation
  (bind _camerarotation (Variables|Camera|GetCameraRotation))
  (bind _cameraoffset (Variables|Camera|GetCameraOffset))
  (Variables|Camera|SetCameraLocation (+ (* (Math|Vector|GetForwardVector _camerarotation) (.x _cameraoffset)) (* (Math|Vector|GetRightVector _camerarotation) (.y _cameraoffset)) (* (Math|Vector|GetUpVector _camerarotation) (.z _cameraoffset)) (.location (Variables|Socket|GetTargetSocket)))))

(fn CalculateContactDistance
  (bind _outhit (Collision|SphereTraceForObjects (.location (Variables|Socket|GetTargetSocket_Target)) (Variables|Camera|GetCameraLocation) (Variables|Camera|GetTraceRadius) (Utilities|Array|MakeArray "ObjectTypeQuery1") false 0 "None"))
  (if (and (.bBlockingHit (Collision|BreakHitResult _outhit)) (not (.bInitialOverlap (Collision|BreakHitResult _outhit))))
    (Variables|Camera|SetCameraLocation (+ (- (.Location (Collision|BreakHitResult _outhit)) (.TraceEnd (Collision|BreakHitResult _outhit))) (Variables|Camera|GetCameraLocation)))))

(fn InterpolateCameraOffset
  (Variables|Camera|SetCameraOffset (Math|Interpolation|VInterpTo (Variables|Camera|GetCameraOffset) (Variables|Camera|GetCameraOffset_Target) (Utilities|Time|GetWorldDeltaSeconds) (Variables|Camera|GetCameraOffset_LagSpeed))))